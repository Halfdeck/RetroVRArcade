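; BP_ArcadeScreen is an in-world arcade monitor that runs a MAME game through a libretro core.
; It plays an attract-mode movie until StartMame loads the core and game, then records the game file in the player state.
; Tick, using a short Delay, feeds inputs, runs the core and applies its texture to the Pane via a new dynamic material.
; KillMame restores the attract movie and unloads the core.
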(event `Create Monitor`
  (params (Texture :type "Texture2D Object Reference"))
  ;[1 1 1] Update Monitor
  (bind _returnvalue (`PrimitiveComponent.CreateDynamicMaterialInstance` (`self.Pane`) 0 "/Game/01_RetroVRArcade/Shared/Materials/ArcadeScreenMat_Inst.ArcadeScreenMat_Inst" "None"))
  (bind _output_get (set `self.DMI_LibretroGame` _returnvalue))
  (`MaterialInstanceDynamic.SetTextureParameterValue` _output_get "TextureToModify" Texture)
  (`PrimitiveComponent.SetMaterial` (`self.Pane`) 0 _output_get))

(event `self.ReceiveBeginPlay`
  ;[1 1 1] Begin Play
  (`self.StartAttractMode`))

(event `StartMame`
  ;[1 1 1] Initialize MAME
  (`self.EnableInput` (`GameplayStatics.GetPlayerController` 0))
  (bind _returnvalue (`self.InitializeCoreV2` "libretro" (`self.DLLFileName`) (`self.GameFileName`)))
  (if _returnvalue
    (set `self.IsGameLoaded` true)
    (`self.CreateTexture` (`self.GameResolutionWidth`) (`self.GameResolutionHeight`))
    (`self.StopAttractMode`)
    (bind _asplayer_state_retro_vr (cast `/Game/01_RetroVRArcade/PlayerState_RetroVR` (`|GetArrayItem` (`GameStateBase.PlayerArray` (`GameplayStatics.GetGameState`)))))
    (set `/Game/01_RetroVRArcade/PlayerState_RetroVR.GameFileName` (`self.GameFileName`) _asplayer_state_retro_vr)))

(event `KillMame`
  ;[1 1 1] Destructor
  (`self.StartAttractMode`)
  (if (`self.IsGameLoaded`)
    (set `self.IsGameLoaded` false)
    (`self.UnloadV2`)))

(event `self.ReceiveTick`
  (params (DeltaSeconds :type "Float (single-precision)"))
  ;[1 1 1] Tick
  (`KismetSystemLibrary.Delay` 0.016)
  (if (`self.IsGameLoaded`)
    (`self.UpdateInputsV2` false)
    (bind _returnvalue (`self.RetroRunV2`))
    (`self.Create Monitor` _returnvalue)))

(event `InputAction|MameConfigMenuSubmit`
  (params (Key :type "Key Structure"))
  ;[1 1 1] Settings Keys
  (:`Pressed`
    (`self.OnKeyPressed` 13))
  (:`Released`
    (`self.OnKeyReleased` 13)))

(event `OnKeyPressed`
  (params (KeyCode :type Integer))
  ;[1 1 1] Update Keypress Array
  (`KismetArrayLibrary.Array_Set` (`self.KeyPresses`) KeyCode true true))

(event `OnKeyReleased`
  (params (KeyCode :type Integer))
  ;[1 1 1] Update Keypress Array
  (`KismetArrayLibrary.Array_Set` (`self.KeyPresses`) KeyCode false true))

(event `InputAction|MameConfigMenu`
  (params (Key :type "Key Structure"))
  ;[1 1 1] Settings Keys
  (:`Pressed`
    (`self.OnKeyPressed` 9))
  (:`Released`
    (`self.OnKeyReleased` 9)))

(event `StartAttractMode`
  ;[1 1 1] Start arcade game attract mode
  (if (not (`MediaPlayer.IsPlaying` (`self.AttractModeMediaPlayer`)))
    (if (`self.IsGameLoaded`)
      (`PrimitiveComponent.SetMaterial` (`self.Pane`) 0 (`self.AttractModeMaterial`)))
    (`MediaPlayer.OpenSource` (`self.AttractModeMediaPlayer`) (`self.AttractModeMediaSource`))))

(event `StopAttractMode`
  ;[1 1 1] Stop arcade game attract mode
  (`MediaPlayer.Close` (`self.AttractModeMediaPlayer`)))

(fn `UserConstructionScript`)